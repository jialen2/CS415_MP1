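; Endless tunnel segment with a spinning holed wall and an optional health pack and enemy.
; When the player reaches the trigger zone, it asks TunnelSpawner for another segment, adds score and destroys itself.
; Overlaps drive player stats: the wall costs score and health, packs heal, enemies damage, and projectiles destroy enemies for destruction score.
; Randomize functions, not called here, vary wall mesh and roll, and give coin-flip chances of placing each item.
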(event OnComponentBeginOverlap(TriggerZone)
  (params (OverlappedComponent :type Primitive%20Component%20Object%20Reference) (OtherActor :type Actor%20Object%20Reference) (OtherComp :type Primitive%20Component%20Object%20Reference) (OtherBodyIndex :type Integer) (bFromSweep :type Boolean) (SweepResult :type Hit%20Result%20Structure%20%28by%20ref%29))
  (bind _healthpack (Variables|Default|GetHealthPack))
  (Utilities|FlowControl|Sequence
    (:then_0
      (Utilities|Casting|CastToBP_Projectile OtherActor))
    (:then_1
      (bind _asbp_player (Utilities|Casting|CastToBP_Player OtherActor))
      (Default|SpawnTunnelatSpawnPoint (Variables|Default|GetTunnelSpawner))
      (bind _output_get (Variables|/Game/InfiniteMatrix/Blueprints/BP_Player.BP_Player_C|SetPlayerScore _asbp_player (+ (Variables|/Game/InfiniteMatrix/Blueprints/BP_Player.BP_Player_C|GetPlayerScore _asbp_player) 1)))
      (Default|UpdateScore (Variables|/Game/InfiniteMatrix/Blueprints/BP_Player.BP_Player_C|GetScoreWidget _asbp_player) _output_get)
      (Actor|DestroyActor)
      (Utilities|FlowControl|Sequence
        (:then_0
          (Utilities|IsValid _healthpack
            (:Is%20Valid
              (Components|DestroyComponent _healthpack))))
        (:then_1
          (Utilities|IsValid (Variables|Default|GetEnemyWidget)
            (:Is%20Valid
              (Components|DestroyComponent (Variables|Default|GetEnemyWidget)))))))))

(event OnComponentBeginOverlap(EnemyWidget)
  (params (OverlappedComponent :type Primitive%20Component%20Object%20Reference) (OtherActor :type Actor%20Object%20Reference) (OtherComp :type Primitive%20Component%20Object%20Reference) (OtherBodyIndex :type Integer) (bFromSweep :type Boolean) (SweepResult :type Hit%20Result%20Structure%20%28by%20ref%29))
  (Utilities|FlowControl|Sequence
    (:then_0
      (bind _asbp_player (Utilities|Casting|CastToBP_Player OtherActor))
      (bind _output_get (Variables|/Game/InfiniteMatrix/Blueprints/BP_Player.BP_Player_C|SetHealth _asbp_player (- (Variables|/Game/InfiniteMatrix/Blueprints/BP_Player.BP_Player_C|GetHealth _asbp_player) 1.0)))
      (Default|UpdateHealthBar (Variables|/Game/InfiniteMatrix/Blueprints/BP_Player.BP_Player_C|GetHealthWidget _asbp_player) _output_get)
      (Components|DestroyComponent (Variables|Default|GetEnemyWidget))
      (if (<= (Variables|/Game/InfiniteMatrix/Blueprints/BP_Player.BP_Player_C|GetHealth _asbp_player) 0.0)
        (Variables|/Game/InfiniteMatrix/Blueprints/BP_Player.BP_Player_C|SetIsDead _asbp_player true)
        (Default|DisplayRestart _asbp_player)))
    (:then_1
      (bind _asbp_projectile (Utilities|Casting|CastToBP_Projectile OtherActor))
      (Variables|/Game/InfiniteMatrix/Blueprints/BP_Player.BP_Player_C|SetDestructionScore (Variables|/Game/InfiniteMatrix/Blueprints/BP_Projectile.BP_Projectile_C|GetPlayer%20 _asbp_projectile) (+ (Variables|/Game/InfiniteMatrix/Blueprints/BP_Player.BP_Player_C|GetDestructionScore (Variables|/Game/InfiniteMatrix/Blueprints/BP_Projectile.BP_Projectile_C|GetPlayer%20 _asbp_projectile)) 1))
      (Default|UpdateDestructionScore (Variables|/Game/InfiniteMatrix/Blueprints/BP_Player.BP_Player_C|GetDestructionWidget (Variables|/Game/InfiniteMatrix/Blueprints/BP_Projectile.BP_Projectile_C|GetPlayer%20 _asbp_projectile)) (+ (Variables|/Game/InfiniteMatrix/Blueprints/BP_Player.BP_Player_C|GetDestructionScore (Variables|/Game/InfiniteMatrix/Blueprints/BP_Projectile.BP_Projectile_C|GetPlayer%20 _asbp_projectile)) 1))
      (Actor|DestroyActor _asbp_projectile)
      (Components|DestroyComponent (Variables|Default|GetEnemyWidget)))))

(event OnComponentBeginOverlap(WallMesh)
  (params (OverlappedComponent :type Primitive%20Component%20Object%20Reference) (OtherActor :type Actor%20Object%20Reference) (OtherComp :type Primitive%20Component%20Object%20Reference) (OtherBodyIndex :type Integer) (bFromSweep :type Boolean) (SweepResult :type Hit%20Result%20Structure%20%28by%20ref%29))
  (Utilities|FlowControl|Sequence
    (:then_0
      (bind _asbp_player (Utilities|Casting|CastToBP_Player OtherActor))
      (bind _output_get (Variables|/Game/InfiniteMatrix/Blueprints/BP_Player.BP_Player_C|SetPlayerScore _asbp_player (- (Variables|/Game/InfiniteMatrix/Blueprints/BP_Player.BP_Player_C|GetPlayerScore _asbp_player) 1)))
      (Default|UpdateScore (Variables|/Game/InfiniteMatrix/Blueprints/BP_Player.BP_Player_C|GetScoreWidget _asbp_player) _output_get)
      (bind _output_get_2 (Variables|/Game/InfiniteMatrix/Blueprints/BP_Player.BP_Player_C|SetHealth _asbp_player (- (Variables|/Game/InfiniteMatrix/Blueprints/BP_Player.BP_Player_C|GetHealth _asbp_player) 1.0)))
      (Default|UpdateHealthBar (Variables|/Game/InfiniteMatrix/Blueprints/BP_Player.BP_Player_C|GetHealthWidget _asbp_player) _output_get_2)
      (if (<= _output_get_2 0.0)
        (Variables|/Game/InfiniteMatrix/Blueprints/BP_Player.BP_Player_C|SetIsDead _asbp_player true)
        (Default|DisplayRestart _asbp_player)))
    (:then_1
      (bind _asbp_projectile (Utilities|Casting|CastToBP_Projectile OtherActor))
      (Actor|DestroyActor _asbp_projectile))))

(event OnComponentBeginOverlap(HealthPack)
  (params (OverlappedComponent :type Primitive%20Component%20Object%20Reference) (OtherActor :type Actor%20Object%20Reference) (OtherComp :type Primitive%20Component%20Object%20Reference) (OtherBodyIndex :type Integer) (bFromSweep :type Boolean) (SweepResult :type Hit%20Result%20Structure%20%28by%20ref%29))
  (Utilities|FlowControl|Sequence
    (:then_0
      (bind _asbp_player (Utilities|Casting|CastToBP_Player OtherActor))
      (if (<= (Variables|/Game/InfiniteMatrix/Blueprints/BP_Player.BP_Player_C|GetHealth _asbp_player) 4.0)
        (bind _output_get (Variables|/Game/InfiniteMatrix/Blueprints/BP_Player.BP_Player_C|SetHealth _asbp_player (+ (Variables|/Game/InfiniteMatrix/Blueprints/BP_Player.BP_Player_C|GetHealth _asbp_player) 1.0)))
        (Default|UpdateHealthBar (Variables|/Game/InfiniteMatrix/Blueprints/BP_Player.BP_Player_C|GetHealthWidget _asbp_player) _output_get)
        (Components|DestroyComponent (Variables|Default|GetHealthPack))))
    (:then_1
      (bind _asbp_projectile (Utilities|Casting|CastToBP_Projectile OtherActor))
      (Actor|DestroyActor _asbp_projectile))))

(event EventBeginPlay)

(event EventTick
  (params (DeltaSeconds :type Float%20%28single-precision%29))
  (Transformation|AddLocalRotation (Variables|Default|GetWallMesh) (Math|Rotator|MakeRotator (* DeltaSeconds (Variables|Default|GetRotateSpeed)) 0.0 0.0) false false))

(fn ConstructionScript)

(fn RandomizeWall
  (Components|StaticMesh|SetStaticMesh (Variables|Default|GetWallMesh) (Utilities|Select :Index (Math|Random|RandomIntegerinRange 0 3) :Option%200 "/Game/InfiniteMatrix/Meshes/SM_Hole_01.SM_Hole_01" :Option%201 "/Game/InfiniteMatrix/Meshes/SM_Hole_02.SM_Hole_02" :Option%202 "/Game/InfiniteMatrix/Meshes/SM_Hole_03.SM_Hole_03" :Option%203 "/Game/InfiniteMatrix/Meshes/SM_Hole_04.SM_Hole_04"))
  (Transformation|AddLocalRotation (Variables|Default|GetWallMesh) (Math|Rotator|MakeRotator (Math|Random|RandomFloatinRange 0.0 3.6e+02) 0.0 0.0) false false))

(fn RandomizeHealthPack
  (if (== (Math|Random|RandomIntegerinRange 1 2) 1)
    (Components|StaticMesh|SetStaticMesh (Variables|Default|GetHealthPack) "/Game/InfiniteMatrix/Meshes/SM_HealthPack.SM_HealthPack")
    (Transformation|AddLocalOffset (Variables|Default|GetHealthPack) (Math|Vector|MakeVector (Math|Random|RandomFloatinRange 2e+02 2.2e+03) (Math|Random|RandomFloatinRange 0.0 3e+02) (Math|Random|RandomFloatinRange 0.0 3e+02)) false false)))

(fn RandomizeEnemy
  (if (== (Math|Random|RandomIntegerinRange 1 2) 2)
    (Components|StaticMesh|SetStaticMesh (Variables|Default|GetEnemyWidget) "/Game/InfiniteMatrix/Meshes/SM_Enemy.SM_Enemy")
    (Transformation|AddLocalOffset (Variables|Default|GetEnemyWidget) (Math|Vector|MakeVector (Math|Random|RandomFloatinRange 2e+02 2.2e+03) (Math|Random|RandomFloatinRange 0.0 3e+02) (Math|Random|RandomFloatinRange 0.0 3e+02)) false false)))